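; One-shot switch actor that shows a door being removed through a cutaway camera when the player touches it.
; The sphere overlap accepts only the first player's pawn, starts the camera sequence, sets IsPressed to block repeats and calls SetGamePaused(false).
; The sequence cuts to CameraToFocus, destroys Door after a delay, then after another delay blends the view back to the player pawn.
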(event `self.Sphere.OnComponentBeginOverlap`
  (params (OverlappedComponent :type "PrimitiveComponent Object Reference") (OtherActor :type "Actor Object Reference") (OtherComp :type "PrimitiveComponent Object Reference") (OtherBodyIndex :type Integer) (bFromSweep :type Boolean) (SweepResult :type "HitResult Structure (by ref)"))
  (if (and (== OtherActor (`GameplayStatics.GetPlayerPawn` 0)) (not (`self.IsPressed`)))
    (`self.CameraSequence`)
    (set `self.IsPressed` true)
    (`GameplayStatics.SetGamePaused` false)))

(event `CameraSequence`
  (`PlayerController.SetViewTargetWithBlend` (`GameplayStatics.GetPlayerController` 0) (`self.CameraToFocus`) 0.0 "VTBlend_Linear" 0.0 false)
  (`KismetSystemLibrary.Delay` 2.0)
  (`self.K2_DestroyActor` (`self.Door`))
  (`KismetSystemLibrary.Delay` 2.0)
  (`self.ReturnToPlayerCam`))

(event `ReturnToPlayerCam`
  (`PlayerController.SetViewTargetWithBlend` (`GameplayStatics.GetPlayerController` 0) (`GameplayStatics.GetPlayerPawn` 0) 2.0 "VTBlend_Linear" 0.0 false))

(fn `UserConstructionScript`)