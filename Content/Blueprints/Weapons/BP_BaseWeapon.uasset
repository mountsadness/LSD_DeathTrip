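; Base hitscan weapon Blueprint for the first-person character, with empty shoot and stop-shooting events, presumably for child weapons to override.
; FireWeapon plays a camera shake, line traces forward from the Linetrace component with debug drawing on, and applies damage to the hit actor.
; Bullet and shell counts live on the player character, cached at BeginPlay; AmmoType selects which count is checked or decremented with a HUD update.
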(event `self.ReceiveBeginPlay`
  (bind _asbp_first_person_character (cast `/Game/FirstPerson/Blueprints/BP_FirstPersonCharacter` (`GameplayStatics.GetPlayerCharacter` 0)))
  (set `self.PlayerCharacterRef` _asbp_first_person_character))

(event `ShootWeapon`)

(event `StopShooting`)

(event `DecreaseAmmo`
  (bind _playercharacterref (`self.PlayerCharacterRef`))
  (bind _playercharacterref_2 (`self.PlayerCharacterRef`))
  (switch `/Game/Blueprints/Weapons/Ammo` (`self.AmmoType`)
    (:`NewEnumerator0`
      (`/Engine/EditorBlueprintResources/StandardMacros.DecrementInt` (`/Game/FirstPerson/Blueprints/BP_FirstPersonCharacter.Bullet` _playercharacterref_2)
        (:`  `
          (`/Game/Blueprints/UI/PlayerHUD.UpdateBulletAmmo` (`/Game/FirstPerson/Blueprints/BP_FirstPersonCharacter.PlayerHUD` _playercharacterref_2)))))
    (:`NewEnumerator1`
      (`/Engine/EditorBlueprintResources/StandardMacros.DecrementInt` (`/Game/FirstPerson/Blueprints/BP_FirstPersonCharacter.Shell` _playercharacterref)
        (:`  `
          (`/Game/Blueprints/UI/PlayerHUD.UpdateShellAmmo` (`/Game/FirstPerson/Blueprints/BP_FirstPersonCharacter.PlayerHUD` _playercharacterref)))))))

(fn `FireWeapon`
  (bind _returnvalue (`SceneComponent.K2_GetComponentLocation` (`self.Linetrace`)))
  ; camer shake
  (`PlayerCameraManager.StartCameraShake` :`self` (`PlayerController.PlayerCameraManager` (`GameplayStatics.GetPlayerController` 0)) :`ShakeClass` (`self.Gun Shake`))
  (bind (_outhit _returnvalue_2) (`KismetSystemLibrary.LineTraceSingleForObjects` _returnvalue (+ _returnvalue (* (`KismetMathLibrary.GetForwardVector` (`SceneComponent.K2_GetComponentRotation` (`self.Linetrace`))) (`self.LinetraceDistance`))) (`|MakeArray` "ObjectTypeQuery1" "ObjectTypeQuery2" "ObjectTypeQuery3" :!type "EObjectTypeQuery Enum") false (`|MakeArray` self (`GameplayStatics.GetPlayerCharacter` 0) :!type "Actor Object Reference") "ForDuration"))
  (if _returnvalue_2
    (`GameplayStatics.ApplyDamage` (`.HitActor` (`GameplayStatics.BreakHitResult` _outhit)) (`self.Base Damage`))))

(fn `HasEnoughAmmo?`
  (returns (HasAmmo :type Boolean))
  (switch `/Game/Blueprints/Weapons/Ammo` (`self.AmmoType`)
    (:`NewEnumerator0`
      (if (> (`/Game/FirstPerson/Blueprints/BP_FirstPersonCharacter.Bullet` (`self.PlayerCharacterRef`)) 0)
        (return true)
        (else
          (return false))))
    (:`NewEnumerator1`
      (if (> (`/Game/FirstPerson/Blueprints/BP_FirstPersonCharacter.Shell` (`self.PlayerCharacterRef`)) 0)
        (return true)
        (else
          (return false))))))

(fn `UserConstructionScript`)