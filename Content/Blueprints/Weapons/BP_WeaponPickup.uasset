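; BP_WeaponPickup is a 2D sprite pickup that gives the first-person character a shotgun or chainsaw on sphere overlap, then destroys itself.
; The construction script uses the Weapon selection to set both the sprite and the weapon class passed to PickupWeapon.
; Tick yaws the actor toward the player like a billboard.
; An endless yo-yo vector tween started on BeginPlay bobs it along an offset.
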(event `self.Sphere.OnComponentBeginOverlap`
  (params (OverlappedComponent :type "PrimitiveComponent Object Reference") (OtherActor :type "Actor Object Reference") (OtherComp :type "PrimitiveComponent Object Reference") (OtherBodyIndex :type Integer) (bFromSweep :type Boolean) (SweepResult :type "HitResult Structure (by ref)"))
  (bind _asbp_first_person_character (cast `/Game/FirstPerson/Blueprints/BP_FirstPersonCharacter` OtherActor))
  (`/Game/FirstPerson/Blueprints/BP_FirstPersonCharacter.PickupWeapon` _asbp_first_person_character (`self.WeaponClass`))
  (`self.K2_DestroyActor`))

(event `self.ReceiveTick`
  (params (DeltaSeconds :type "Float (single-precision)"))
  (bind (_returnvalue_roll _returnvalue_pitch _returnvalue_yaw) (`KismetMathLibrary.BreakRotator` (`KismetMathLibrary.FindLookAtRotation` (`self.K2_GetActorLocation`) (`self.K2_GetActorLocation` (`GameplayStatics.GetPlayerCharacter` 0)))))
  (`self.K2_SetActorRotation` (`KismetMathLibrary.MakeRotator` 0.0 0.0 _returnvalue_yaw)))

(event `self.ReceiveBeginPlay`
  (bind _returnvalue (`self.K2_GetActorLocation`))
  ; for movement up and down
  (bind (_asynctaskproxy _value) (`FCTweenBPActionVector.TweenVector` _returnvalue (+ _returnvalue (`self.Offset`)) (`self.Duration Secs`) "InOutQuad" 0.0 0.0 0.0 -1 0.0 true)
    (:`ApplyEasing`
      (`self.K2_SetActorLocation` _value))))

(fn `UserConstructionScript`
  (switch `/Game/Blueprints/Weapons/Weapons` (`self.Weapon`)
    (:`NewEnumerator0`
      (`PaperSpriteComponent.SetSprite` (`self.PaperSprite`) "/Game/RetroFPSAssets/Weapons/Shotgun/ShotgunSprite.ShotgunSprite")
      (set `self.WeaponClass` "/Game/Blueprints/Weapons/BP_Shotgun.BP_Shotgun_C"))
    (:`NewEnumerator1`
      (`PaperSpriteComponent.SetSprite` (`self.PaperSprite`) "/Game/RetroFPSAssets/Weapons/Chainsaw/SawPickup.SawPickup")
      (set `self.WeaponClass` "/Game/Blueprints/Weapons/BP_Chainsaw.BP_Chainsaw_C"))))