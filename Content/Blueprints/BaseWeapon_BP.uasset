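; Base weapon Blueprint providing hitscan firing and ammo handling for the first-person character.
; FireWeapon line traces from the Line component, ending at its scaled forward vector offset by NewVar rather than the start location, and applies damage to the hit actor.
; HasAmmo and DecreaseAmmo use AmmoType to select the player's Bullet or Shell count, with decrements also refreshing the player's widget.
; The player reference is cached on BeginPlay.
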(event `DecreaseAmmo`
  (bind _player_ref (`self.Player_Ref`))
  (bind _player_ref_2 (`self.Player_Ref`))
  (switch `/Game/Blueprints/AmmoEnum` (`self.Ammo_Type`)
    (:`NewEnumerator0`
      (`/Engine/EditorBlueprintResources/StandardMacros.DecrementInt` (`/Game/FirstPerson/Blueprints/BP_FirstPersonCharacter.Bullet` _player_ref_2)
        (:`  `
          (`/Game/Blueprints/UI_BP.UpdateBullets` (`/Game/FirstPerson/Blueprints/BP_FirstPersonCharacter.Widgetzzz` _player_ref_2)))))
    (:`NewEnumerator1`
      (`/Engine/EditorBlueprintResources/StandardMacros.DecrementInt` (`/Game/FirstPerson/Blueprints/BP_FirstPersonCharacter.Shell` _player_ref)
        (:`  `
          (`/Game/Blueprints/UI_BP.UpdateShells` (`/Game/FirstPerson/Blueprints/BP_FirstPersonCharacter.Widgetzzz` _player_ref)))))))

(event `self.ReceiveBeginPlay`
  (bind _asbp_first_person_character (cast `/Game/FirstPerson/Blueprints/BP_FirstPersonCharacter` (`GameplayStatics.GetPlayerCharacter` 0)))
  (set `self.Player_Ref` _asbp_first_person_character))

(fn `FireWeapon`
  (locals (NewLocalVar :type "/Game/Blueprints/BaseWeapon_BP Object Reference") (NewLocalVar_0 :type "PlayerController Object Reference"))
  (bind _line (`self.Line`))
  (bind (_outhit _returnvalue) (`KismetSystemLibrary.LineTraceSingleForObjects` (`SceneComponent.K2_GetComponentLocation` _line) (+ (* (`KismetMathLibrary.GetForwardVector` (`SceneComponent.K2_GetComponentRotation` _line)) (`self.Firedistance`)) (`self.NewVar`)) (`|MakeArray` "ObjectTypeQuery1" "ObjectTypeQuery2" "ObjectTypeQuery3" :!type "EObjectTypeQuery Enum") false (`|MakeArray` self (`GameplayStatics.GetPlayerController` 0) :!type "Actor Object Reference")))
  (if _returnvalue
    (`GameplayStatics.ApplyDamage` (`.HitActor` (`GameplayStatics.BreakHitResult` _outhit)) (`self.WeaponDamage`))))

(fn `Has Ammo?`
  (returns (`Has bullets` :type Boolean))
  ;[0.01132 0.15 0 0.5] Witch ammo
  (switch `/Game/Blueprints/AmmoEnum` (`self.Ammo_Type`)
    (:`NewEnumerator0`
      ;[0 0.15 0.1394 0.5] Bullet
      (if (> (`/Game/FirstPerson/Blueprints/BP_FirstPersonCharacter.Bullet` (`self.Player_Ref`)) 0.0)
        (return true)
        (else
          (return false))))
    (:`NewEnumerator1`
      ;[0.15 0 0.00678 0.5] Shell
      (if (> (`/Game/FirstPerson/Blueprints/BP_FirstPersonCharacter.Shell` (`self.Player_Ref`)) 0)
        (return true)
        (else
          (return false))))))

(fn `UserConstructionScript`)