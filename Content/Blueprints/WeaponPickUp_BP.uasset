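; Weapon pickup actor that gives the first-person player a pistol or shotgun.
; The construction script uses the weapon type to set the sprite and the weapon class to grant.
; Each tick it yaws toward the player like a billboard.
; When the first-person character overlaps its sphere, it passes the class to that character's pickup function and destroys itself.
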(event `self.ReceiveTick`
  (params (DeltaSeconds :type "Float (single-precision)"))
  (bind (_returnvalue_roll _returnvalue_pitch _returnvalue_yaw) (`KismetMathLibrary.BreakRotator` (`KismetMathLibrary.FindLookAtRotation` (`self.K2_GetActorLocation`) (`self.K2_GetActorLocation` (`GameplayStatics.GetPlayerCharacter` 0)))))
  (`self.K2_SetActorRotation` (`KismetMathLibrary.MakeRotator` 0.0 0.0 _returnvalue_yaw)))

(event `self.Sphere.OnComponentBeginOverlap`
  (params (OverlappedComponent :type "PrimitiveComponent Object Reference") (OtherActor :type "Actor Object Reference") (OtherComp :type "PrimitiveComponent Object Reference") (OtherBodyIndex :type Integer) (bFromSweep :type Boolean) (SweepResult :type "HitResult Structure (by ref)"))
  (bind _asbp_first_person_character (cast `/Game/FirstPerson/Blueprints/BP_FirstPersonCharacter` OtherActor))
  (`/Game/FirstPerson/Blueprints/BP_FirstPersonCharacter.PickUpWeapon` _asbp_first_person_character (`self.WeaponClass`))
  (`self.K2_DestroyActor`))

(fn `UserConstructionScript`
  (switch `/Game/Blueprints/Weapons_Enum` (`self.WeaponType`)
    (:`NewEnumerator0`
      (`PaperSpriteComponent.SetSprite` (`self.sgn2a0_Sprite_0`) "/Game/RetroFPSAssets/Weapons/Pistol/pistol1_Sprite.pistol1_Sprite")
      (set `self.WeaponClass` "/Game/Blueprints/Pistol_BP.Pistol_BP_C"))
    (:`NewEnumerator1`
      (`PaperSpriteComponent.SetSprite` (`self.sgn2a0_Sprite_0`) "/Game/RetroFPSAssets/Weapons/Shotgun/sgn2a0_Sprite_0.sgn2a0_Sprite_0")
      (set `self.WeaponClass` "/Game/Blueprints/Shotgun_BP.Shotgun_BP_C"))))