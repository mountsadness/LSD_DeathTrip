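; Pistol weapon Blueprint, a child class that fires when ammo is available and animates a Paper2D flipbook.
; A DoOnce gate limits firing: it decreases ammo, plays the shoot flipbook for its length, returns to idle, then resets.
; A dynamic sprite material, noted as for the enemy, supports an unfinished flicker on the E key that only zeroes TintMask and reads it back.
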(event `self.FireWeapon`
  (bind _paperflipbook (`self.PaperFlipbook`))
  ;[0.15 0.007132 0.05993 0.5] Fire weapon
  (bind _has_bullets (`self.Has Ammo?`))
  (if _has_bullets
    (`/Engine/EditorBlueprintResources/StandardMacros.DoOnce` false :!label _label
      (:`Completed`
        (`self.DecreaseAmmo`)
        (`self.FireWeapon`)
        (`PaperFlipbookComponent.SetFlipbook` _paperflipbook "/Game/RetroFPSAssets/Weapons/Pistol/pistolShoot.pistolShoot")
        (`KismetSystemLibrary.Delay` (`PaperFlipbookComponent.GetFlipbookLength` _paperflipbook))
        (`PaperFlipbookComponent.SetFlipbook` (`self.PaperFlipbook`) "/Game/RetroFPSAssets/Weapons/Pistol/pistolIdle.pistolIdle")
        (`self.Resset`)))))

(event `Resset`
  ;[0.15 0.007132 0.05993 0.5] Fire weapon
  (goto _label :!via `Reset`))

(event `CreateRuntimeMaterial`
  ;[0.06938 0.001939 0.15 0.5] This is for the enemy
  (bind _returnvalue (`PrimitiveComponent.CreateDynamicMaterialInstance` (`self.PaperFlipbook`) 0 "/Game/FirstPerson/Materials/MM_SpriteMaterial.MM_SpriteMaterial" "None"))
  (set `self.runtimeMat` _returnvalue))

(event `Key|E`
  (params (Key :type "Key Structure"))
  ;[0 0.4739 0.2841 0.5] for inputs
  (:`Pressed`
    (`self.Flickr`)))

(event `Flickr`
  ;[0.06938 0.001939 0.15 0.5] This is for the enemy
  ;; set mask to 0
  (`MaterialInstanceDynamic.SetScalarParameterValue` (`self.runtimeMat`) (`self.TintMask`) 0.0)
  ;; initial value from mask
  (`MaterialInstanceDynamic.K2_GetScalarParameterValue` (`self.runtimeMat`) (`self.TintMask`)))

(fn `UserConstructionScript`
  (`parent.UserConstructionScript`))