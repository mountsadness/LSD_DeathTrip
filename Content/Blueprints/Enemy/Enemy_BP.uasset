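; Enemy_BP is an AI enemy drawn as a Paper2D flipbook that senses the player, attacks by melee or projectile, takes damage and dies.
; Tick derives an animation state from velocity and attack flags, then sets flipbook and relative rotation from the player's angle via dot products.
; Pawn sensing drives turning and the CanSeePlayer blackboard key, cleared by retriggerable delay.
; Melee uses a line trace; death stops AI, movement and collision.
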(event `self.ReceiveTick`
  (params (DeltaSeconds :type "Float (single-precision)"))
  (bind _returnvalue (`KismetMathLibrary.Normal` (- (`self.K2_GetActorLocation` (`GameplayStatics.GetPlayerCharacter` 0)) (`self.K2_GetActorLocation`))))
  (if (< (`KismetMathLibrary.VSize` (`MovementComponent.Velocity` (`self.CharacterMovement`))) 0.0)
    (if (`self.IsAttacking`)
      (switch `/Game/Blueprints/Enemy/AttackState` (`self.EnemyAttack`)
        (:`NewEnumerator0`
          (set `self.EnemyState` "NewEnumerator2"))
        (:`NewEnumerator1`
          (set `self.EnemyState` "NewEnumerator2")))
      (else
        (set `self.EnemyState` "NewEnumerator1")))
    (elif (`self.IsAttacking`)
      (switch `/Game/Blueprints/Enemy/AttackState` (`self.EnemyAttack`)
        (:`NewEnumerator0`
          (set `self.EnemyState` "NewEnumerator2"))
        (:`NewEnumerator1`
          (set `self.EnemyState` "NewEnumerator3")))
      (else
        (set `self.EnemyState` "NewEnumerator0"))))
  (if (`self.IsDead`)
    (`self.HandleDead`)
    (else
      (if (`self.CanSeePlayer`)
        (`self.RotateTowardsPlayer`))
      (bind _output_get (set `self.Degrees` (`KismetMathLibrary.DegAcos` (`KismetMathLibrary.Dot_VectorVector` (`self.GetActorForwardVector`) _returnvalue))))
      (if (< (`KismetMathLibrary.Dot_VectorVector` (`self.GetActorRightVector`) _returnvalue) 0.0)
        (`/Engine/EditorBlueprintResources/StandardMacros.CompareFloat` (`self.Degrees`) 180.0
          (:`>`
            (`SceneComponent.K2_SetRelativeRotation` (`self.PaperFlipbook`) (struct :`Yaw` -90.0) false false :!label _label)
            (`PaperFlipbookComponent.SetFlipbook` (`self.PaperFlipbook`) (`|GetArrayItem` (select `/Game/Blueprints/Enemy/EnemyState` (`self.EnemyState`) :`NewEnumerator0` (`self.IdleFlipbook`) :`NewEnumerator1` (`self.MoveFlipbook`) :`NewEnumerator2` (`self.MeleeFlipbook`) :`NewEnumerator3` (`self.ShootFlipbook`)))))
          (:`==`
            (goto _label))
          (:`<`
            (`/Engine/EditorBlueprintResources/StandardMacros.CompareFloat` (`self.Degrees`) _output_get
              (:`>`
                (`SceneComponent.K2_SetRelativeRotation` (`self.PaperFlipbook`) (struct :`Yaw` 135.0) false false :!label _label_2)
                (`PaperFlipbookComponent.SetFlipbook` (`self.PaperFlipbook`) (`|GetArrayItem` (select `/Game/Blueprints/Enemy/EnemyState` (`self.EnemyState`) :`NewEnumerator0` (`self.IdleFlipbook`) :`NewEnumerator1` (`self.MoveFlipbook`) :`NewEnumerator2` (`self.MeleeFlipbook`) :`NewEnumerator3` (`self.ShootFlipbook`)))))
              (:`==`
                (goto _label_2))
              (:`<`
                (`/Engine/EditorBlueprintResources/StandardMacros.CompareFloat` (`self.Degrees`) 90.0
                  (:`>`
                    (`SceneComponent.K2_SetRelativeRotation` (`self.PaperFlipbook`) (struct :`Yaw` 180.0) false false :!label _label_3)
                    (`PaperFlipbookComponent.SetFlipbook` (`self.PaperFlipbook`) (`|GetArrayItem` (select `/Game/Blueprints/Enemy/EnemyState` (`self.EnemyState`) :`NewEnumerator0` (`self.IdleFlipbook`) :`NewEnumerator1` (`self.MoveFlipbook`) :`NewEnumerator2` (`self.MeleeFlipbook`) :`NewEnumerator3` (`self.ShootFlipbook`)))))
                  (:`==`
                    (goto _label_3))
                  (:`<`
                    (`/Engine/EditorBlueprintResources/StandardMacros.CompareFloat` (`self.Degrees`) 45.0
                      (:`>`
                        _)
                      (:`==`
                        _)
                      (:`<`
                        (goto _label)))
                    (`SceneComponent.K2_SetRelativeRotation` (`self.PaperFlipbook`) (struct :`Yaw` 45.0) false false)
                    (`PaperFlipbookComponent.SetFlipbook` (`self.PaperFlipbook`) (`|GetArrayItem` (select `/Game/Blueprints/Enemy/EnemyState` (`self.EnemyState`) :`NewEnumerator0` (`self.IdleFlipbook`) :`NewEnumerator1` (`self.MoveFlipbook`) :`NewEnumerator2` (`self.MeleeFlipbook`) :`NewEnumerator3` (`self.ShootFlipbook`))))))))))
        (else
          (`/Engine/EditorBlueprintResources/StandardMacros.CompareFloat` (`self.Degrees`) 180.0
            (:`>`
              (`SceneComponent.K2_SetRelativeRotation` (`self.PaperFlipbook`) (struct :`Yaw` -45.0) false false :!label _label_4)
              (`PaperFlipbookComponent.SetFlipbook` (`self.PaperFlipbook`) (`|GetArrayItem` (select `/Game/Blueprints/Enemy/EnemyState` (`self.EnemyState`) :`NewEnumerator0` (`self.IdleFlipbook`) :`NewEnumerator1` (`self.MoveFlipbook`) :`NewEnumerator2` (`self.MeleeFlipbook`) :`NewEnumerator3` (`self.ShootFlipbook`)))))
            (:`==`
              (goto _label_4))
            (:`<`
              (`/Engine/EditorBlueprintResources/StandardMacros.CompareFloat` (`self.Degrees`) 135.0
                (:`>`
                  (`SceneComponent.K2_SetRelativeRotation` (`self.PaperFlipbook`) (struct :`Yaw` 90.0) false false :!label _label_5)
                  (`PaperFlipbookComponent.SetFlipbook` (`self.PaperFlipbook`) (`|GetArrayItem` (select `/Game/Blueprints/Enemy/EnemyState` (`self.EnemyState`) :`NewEnumerator0` (`self.IdleFlipbook`) :`NewEnumerator1` (`self.MoveFlipbook`) :`NewEnumerator2` (`self.MeleeFlipbook`) :`NewEnumerator3` (`self.ShootFlipbook`)))))
                (:`==`
                  (goto _label_5))
                (:`<`
                  (`/Engine/EditorBlueprintResources/StandardMacros.CompareFloat` (`self.Degrees`) 90.0
                    (:`>`
                      (`SceneComponent.K2_SetRelativeRotation` (`self.PaperFlipbook`) (struct :`Yaw` 45.0) false false :!label _label_6)
                      (`PaperFlipbookComponent.SetFlipbook` (`self.PaperFlipbook`) (`|GetArrayItem` (select `/Game/Blueprints/Enemy/EnemyState` (`self.EnemyState`) :`NewEnumerator0` (`self.IdleFlipbook`) :`NewEnumerator1` (`self.MoveFlipbook`) :`NewEnumerator2` (`self.MeleeFlipbook`) :`NewEnumerator3` (`self.ShootFlipbook`)))))
                    (:`==`
                      (goto _label_6))
                    (:`<`
                      (`/Engine/EditorBlueprintResources/StandardMacros.CompareFloat` (`self.Degrees`) 45.0
                        (:`>`
                          _)
                        (:`==`
                          _)
                        (:`<`
                          (goto _label_4)))
                      (`SceneComponent.K2_SetRelativeRotation` :`self` (`self.PaperFlipbook`))
                      (`PaperFlipbookComponent.SetFlipbook` (`self.PaperFlipbook`) (`|GetArrayItem` (select `/Game/Blueprints/Enemy/EnemyState` (`self.EnemyState`) :`NewEnumerator0` (`self.IdleFlipbook`) :`NewEnumerator1` (`self.MoveFlipbook`) :`NewEnumerator2` (`self.MeleeFlipbook`) :`NewEnumerator3` (`self.ShootFlipbook`)))))))))))))))

(event `RotateTowardsPlayer`
  (`self.K2_SetActorRotation` (`KismetMathLibrary.RInterpTo` (`self.K2_GetActorRotation`) (`KismetMathLibrary.FindLookAtRotation` (`self.K2_GetActorLocation`) (`self.K2_GetActorLocation` (`GameplayStatics.GetPlayerCharacter` 0))) (`GameplayStatics.GetWorldDeltaSeconds`) 10.0)))

(event `self.PawnSensing.OnSeePawn`
  (params (Pawn :type "Pawn Object Reference"))
  (cast `/Game/FirstPerson/Blueprints/BP_FirstPersonCharacter` Pawn)
  (set `self.CanSeePlayer` true)
  (`BlackboardComponent.SetValueAsBool` (`AIBlueprintHelperLibrary.GetBlackboard` null) "CanSeePlayer" true)
  (`KismetSystemLibrary.RetriggerableDelay` 0.7)
  (set `self.CanSeePlayer` false)
  (`BlackboardComponent.SetValueAsBool` (`AIBlueprintHelperLibrary.GetBlackboard` null) "CanSeePlayer" false))

(event `SpawnProjectile`
  (set `self.IsAttacking` true)
  (set `self.EnemyAttack` "NewEnumerator1")
  (`MovementComponent.StopMovementImmediately` (`self.CharacterMovement`))
  (`KismetSystemLibrary.RetriggerableDelay` 0.2)
  (`|SpawnActorFromClass` "/Game/Blueprints/Enemy/EnemyBullet_BP.EnemyBullet_BP_C" (`SceneComponent.K2_GetComponentToWorld` (`self.SpawnPoint`)) "Undefined" "MultiplyWithRoot" null null)
  (set `self.IsAttacking` false))

(event `MeleeAttack`
  (bind _returnvalue (`self.K2_GetActorLocation`))
  ; Damage Player
  (set `self.IsAttacking` true)
  (set `self.EnemyAttack` "NewEnumerator0")
  (`KismetSystemLibrary.RetriggerableDelay` 0.5)
  (bind _outhit (`KismetSystemLibrary.LineTraceSingleForObjects` _returnvalue (+ _returnvalue (* (`self.GetActorForwardVector`) 200.0)) (`|MakeArray` "ObjectTypeQuery3" :!type "EObjectTypeQuery Enum") false (`|MakeArray` self :!type "Actor Object Reference")))
  (bind (_bblockinghit _binitialoverlap _time _distance _location _impactpoint _normal _impactnormal _physmat _hitactor) (`GameplayStatics.BreakHitResult` _outhit))
  (if (== _hitactor (`GameplayStatics.GetPlayerCharacter` 0))
    (`GameplayStatics.ApplyDamage` _hitactor 50.0)))

(event `self.ReceiveAnyDamage`
  (params (Damage :type "Float (single-precision)") (DamageType :type "DamageType Object Reference") (InstigatedBy :type "Controller Object Reference") (DamageCauser :type "Actor Object Reference"))
  (`PaperFlipbookComponent.SetSpriteColor` (`self.PaperFlipbook`) (struct :`R` 1.0 :`A` 1.0))
  (`KismetSystemLibrary.Delay` 0.1)
  (`PaperFlipbookComponent.SetSpriteColor` (`self.PaperFlipbook`) (struct :`R` 1.0 :`G` 1.0 :`B` 1.0 :`A` 1.0))
  (bind _output_get (set `self.health` (- (`self.health`) Damage)))
  (if (<= _output_get 0.0)
    (set `self.IsDead` true)))

(event `HandleDead`
  (bind _paperflipbook (`self.PaperFlipbook`))
  (bind (_returnvalue_roll _returnvalue_pitch _returnvalue_yaw) (`KismetMathLibrary.BreakRotator` (`KismetMathLibrary.FindLookAtRotation` (`self.K2_GetActorLocation`) (`self.K2_GetActorLocation` (`GameplayStatics.GetPlayerController` 0)))))
  (`self.K2_SetActorRotation` (`KismetMathLibrary.MakeRotator` 0.0 0.0 _returnvalue_yaw))
  (`/Engine/EditorBlueprintResources/StandardMacros.DoOnce` false
    (:`Completed`
      (`BrainComponent.StopLogic` (`AIController.BrainComponent` (`AIBlueprintHelperLibrary.GetAIController` self)) "")
      (`CharacterMovementComponent.SetMovementMode` (`self.CharacterMovement`) "MOVE_None" 0)
      (`PrimitiveComponent.SetCollisionEnabled` (`self.CapsuleComponent`) "NoCollision")
      (`ActorComponent.Deactivate` (`self.CharacterMovement`))
      (`SceneComponent.K2_SetRelativeRotation` :`self` _paperflipbook)
      (`PaperFlipbookComponent.SetFlipbook` _paperflipbook null)
      (`KismetSystemLibrary.Delay` (- (`PaperFlipbookComponent.GetFlipbookLength` _paperflipbook) 0.0))
      (`self.K2_AddActorLocalOffset` (0.0 0.0 0.0))
      (`PaperFlipbookComponent.SetFlipbook` (`self.PaperFlipbook`) null))))

(fn `UserConstructionScript`)