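; BP_KeyCard is a collectible keycard pickup that spins continuously and bobs up and down in the level.
; Tick adds a small local rotation, while BeginPlay starts an endlessly looping yoyo TweenVector between the start location and an Offset to drive the movement.
; When the player pawn overlaps the Sphere, it sets HasKey on BP_FirstPersonCharacter and destroys itself.
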(event `self.ReceiveTick`
  (params (DeltaSeconds :type "Float (single-precision)"))
  ; rotation
  (`self.K2_AddActorLocalRotation` (struct :`Yaw` 0.5)))

(event `self.ReceiveBeginPlay`
  (bind _returnvalue (`self.K2_GetActorLocation`))
  ; for movement up and down
  (bind (_asynctaskproxy _value) (`FCTweenBPActionVector.TweenVector` _returnvalue (+ _returnvalue (`self.Offset`)) 1.0 "InOutQuad" 0.0 0.0 0.0 -1 0.0 true)
    (:`ApplyEasing`
      (`self.K2_SetActorLocation` _value))))

(event `self.Sphere.OnComponentBeginOverlap`
  (params (OverlappedComponent :type "PrimitiveComponent Object Reference") (OtherActor :type "Actor Object Reference") (OtherComp :type "PrimitiveComponent Object Reference") (OtherBodyIndex :type Integer) (bFromSweep :type Boolean) (SweepResult :type "HitResult Structure (by ref)"))
  ; destroy key card
  (if (== OtherActor (`GameplayStatics.GetPlayerPawn` 0))
    (bind _asbp_first_person_character (cast `/Game/FirstPerson/Blueprints/BP_FirstPersonCharacter` (`GameplayStatics.GetPlayerPawn` 0)))
    (set `/Game/FirstPerson/Blueprints/BP_FirstPersonCharacter.HasKey` true _asbp_first_person_character)
    (`self.K2_DestroyActor`)))

(fn `UserConstructionScript`)