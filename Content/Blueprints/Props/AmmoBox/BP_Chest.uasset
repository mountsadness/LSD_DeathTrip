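; BP_Chest is an ammo chest that gives the first-person player bullets and shells when E is pressed within range, and is reusable.
; A sphere overlap sets the range flag, though its end-overlap check compares the overlapped component to the pawn rather than the other actor.
; A yoyo rotator tween with easing swings the lid, while CanInteract blocks retriggering until the tween completes.
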(event `Key|E` :consume false
  (params (Key :type "Key Structure"))
  ; OPEN AND CLOSE CHEST
  (:`Pressed`
    (`self.OpenChest`)))

(event `OpenChest`
  (bind _player (`self.Player`))
  (bind _relativerotation (`SceneComponent.RelativeRotation` (`self.SM_ChestLid`)))
  ; OPEN AND CLOSE CHEST
  (if (and (`self.playerinRange`) (`self.canInteract`))
    (bind (_asynctaskproxy _value) (`FCTweenBPActionRotator.TweenRotator` _relativerotation (`KismetMathLibrary.ComposeRotators` _relativerotation (`self.offsetRotation`)) (`self.openTile`) "InOutQuad" 0.0 0.0 0.0 1 0.0 true)
      (:`then`
        (set `self.canInteract` false)
        (`/Game/FirstPerson/Blueprints/BP_FirstPersonCharacter.AddBullets` _player 50)
        (`/Game/FirstPerson/Blueprints/BP_FirstPersonCharacter.AddShells` _player 30))
      (:`ApplyEasing`
        (`SceneComponent.K2_SetRelativeRotation` (`self.SM_ChestLid`) _value false false))
      (:`OnComplete`
        (set `self.canInteract` true)))))

(event `self.ReceiveBeginPlay`
  ; chest is interactable
  (set `self.canInteract` true)
  (bind _asbp_first_person_character (cast `/Game/FirstPerson/Blueprints/BP_FirstPersonCharacter` (`GameplayStatics.GetPlayerPawn` 0)))
  (set `self.Player` _asbp_first_person_character))

(event `self.Sphere.OnComponentBeginOverlap`
  (params (OverlappedComponent :type "PrimitiveComponent Object Reference") (OtherActor :type "Actor Object Reference") (OtherComp :type "PrimitiveComponent Object Reference") (OtherBodyIndex :type Integer) (bFromSweep :type Boolean) (SweepResult :type "HitResult Structure (by ref)"))
  ; It detrmin if player is in range or not
  (if (== OtherActor (`GameplayStatics.GetPlayerPawn` 0))
    (set `self.playerinRange` true)))

(event `self.Sphere.OnComponentEndOverlap`
  (params (OverlappedComponent :type "PrimitiveComponent Object Reference") (OtherActor :type "Actor Object Reference") (OtherComp :type "PrimitiveComponent Object Reference") (OtherBodyIndex :type Integer))
  ; It detrmin if player is in range or not
  (if (== OverlappedComponent (`GameplayStatics.GetPlayerPawn` 0))
    (set `self.playerinRange` false)))

(fn `UserConstructionScript`)