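; BP_Switch is a prop trigger that briefly switches the player's view to a focus camera, commented as showing a door.
; When the player pawn overlaps its Box, CameraSquence sets the view target to CameraToFocus, then returns it to the controlled pawn after a short delay.
; The IsPressd guard is only ever set to false here, so the sequence can retrigger on each overlap.
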(event `Camera Squence`
  ; Camera showing door
  (`PlayerController.SetViewTargetWithBlend` (`GameplayStatics.GetPlayerController` 0) (`self.cameraToFocus`) 0.0 "VTBlend_Linear" 0.0 false)
  (`KismetSystemLibrary.Delay` 1.0)
  (`self.ReturnToPlayerCam`))

(event `ReturnToPlayerCam`
  (bind _returnvalue (`GameplayStatics.GetPlayerController` 0))
  (`PlayerController.SetViewTargetWithBlend` _returnvalue (`Controller.K2_GetPawn` _returnvalue) 0.0 "VTBlend_Linear" 0.0 false))

(event `self.Box.OnComponentBeginOverlap`
  (params (OverlappedComponent :type "PrimitiveComponent Object Reference") (OtherActor :type "Actor Object Reference") (OtherComp :type "PrimitiveComponent Object Reference") (OtherBodyIndex :type Integer) (bFromSweep :type Boolean) (SweepResult :type "HitResult Structure (by ref)"))
  ; Is pressed
  (if (and (== OtherActor (`GameplayStatics.GetPlayerPawn` 0)) (not (`self.isPressd`)))
    (`self.Camera Squence`)
    (set `self.isPressd` false)
    (`GameplayStatics.SetGamePaused` false)))

(fn `UserConstructionScript`)