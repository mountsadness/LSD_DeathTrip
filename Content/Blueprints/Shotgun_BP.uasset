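; Shotgun weapon Blueprint that fires when it has ammo and animates the shot with Paper2D flipbooks.
; FireWeapon passes a DoOnce gate, spends ammo, calls FireWeapon and switches to the Shotgun1 flipbook.
; After a delay taken from the flipbook's length, it switches to Shotgun2 and calls Resset to reopen the gate, blocking refire during the animation.
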(event `self.FireWeapon`
  (bind _paperflipbook (`self.PaperFlipbook`))
  (bind _has_bullets (`self.Has Ammo?`))
  (if _has_bullets
    (`/Engine/EditorBlueprintResources/StandardMacros.DoOnce` false :!label _label
      (:`Completed`
        (`self.DecreaseAmmo`)
        (`self.FireWeapon`)
        (`PaperFlipbookComponent.SetFlipbook` _paperflipbook "/Game/RetroFPSAssets/Weapons/Shotgun/shotgun1.shotgun1")
        (`KismetSystemLibrary.Delay` (`PaperFlipbookComponent.GetFlipbookLength` _paperflipbook))
        (`PaperFlipbookComponent.SetFlipbook` (`self.PaperFlipbook`) "/Game/RetroFPSAssets/Weapons/Shotgun/shotgun2.shotgun2")
        (`self.Resset`)))))

(event `Resset`
  (goto _label :!via `Reset`))

(fn `UserConstructionScript`
  (`parent.UserConstructionScript`))